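; BP_PartolAI is an AI pawn that chases the player character, despite its patrol naming.
; On BeginPlay it prints the count of actors tagged as test patrol points, which are not used for movement, then starts the MoveTo event.
; MoveTo runs AIMoveTo toward the player, prints success or failure, and calls itself again after a short delay, forming an endless follow loop.
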(event `self.ReceiveBeginPlay`
  (bind _outactors (`GameplayStatics.GetAllActorsOfClassWithTag` "/Script/Engine.Actor" "PatrolPoint-testpoint"))
  (`KismetSystemLibrary.PrintString` (`KismetStringLibrary.Concat_StrStr` "There are " (`KismetStringLibrary.Conv_IntToString` (`KismetArrayLibrary.Array_Length` _outactors)) "patrol points."))
  (`self.Move to`))

(event `Move to`
  (`|AIMoveTo` self (0.0 0.0 0.0) (`GameplayStatics.GetPlayerCharacter` 0) 50.0 ; move ourselves to the players location, constantly updating
    (:`OnSuccess`
      (`KismetSystemLibrary.PrintString` "arrived at you"))
    (:`OnFail`
      (`KismetSystemLibrary.PrintString` "failed")))
  (`KismetSystemLibrary.Delay` 1.0)
  (`self.Move to`))

(fn `UserConstructionScript`)