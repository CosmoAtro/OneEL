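; BP_GrayBoar is an enemy boar that wanders the navmesh and chases pawns it sees.
; Roaming chains AI MoveTo calls to random navigable points around its location.
; PawnSensing sightings start a move toward the pawn, with a DoOnce switching to run animation and sprint speed once.
; A retriggerable delay, refreshed by each sighting, restores walking, resets the DoOnce and resumes roaming after sight is lost.
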(event `self.ReceiveBeginPlay`
  ;[1 1 1] Walks
  (`self.Movetorandomlocation`))

(event `Movetorandomlocation`
  ;[1 1 1] Walks
  (bind _randomlocation (`NavigationSystemV1.K2_GetRandomLocationInNavigableRadius` (`self.K2_GetActorLocation`) 0.0 null null))
  (`|AIMoveTo` self _randomlocation null
    (:`OnSuccess`
      (`self.Movetorandomlocation`))))

(event `CanSprintAgain`
  ;[1 1 1] Chase
  (goto _label :!via `Reset`))

(event `self.PawnSensing.OnSeePawn`
  (params (Pawn :type "Pawn Object Reference"))
  ;[1 1 1] Chase
  (`|ExecutionSequence`
    (:`then_0`
      (`/Engine/EditorBlueprintResources/StandardMacros.DoOnce` false :!label _label
        (:`Completed`
          (`SkeletalMeshComponent.PlayAnimation` (`self.Mesh`) "/Game/StylizedCreaturesBundle/Animations/Boar/A_Boar_Run_Forward.A_Boar_Run_Forward" true)
          (set `CharacterMovementComponent.MaxWalkSpeed` 600.0 (`self.CharacterMovement`)))))
    (:`then_1`
      (`|AIMoveTo` self (0.0 0.0 0.0) Pawn
        (:`then`
          ;[1 1 1] Stops chase when we hide
          (`KismetSystemLibrary.RetriggerableDelay` 2.0)
          (`SkeletalMeshComponent.PlayAnimation` (`self.Mesh`) "/Game/StylizedCreaturesBundle/Animations/Boar/A_Boar_Walk_Forward.A_Boar_Walk_Forward" true)
          (set `CharacterMovementComponent.MaxWalkSpeed` 300.0 (`self.CharacterMovement`))
          (`self.CanSprintAgain`)
          (`self.Movetorandomlocation`))))))

(fn `UserConstructionScript`)