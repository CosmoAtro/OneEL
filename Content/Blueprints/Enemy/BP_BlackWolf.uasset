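; Black wolf enemy that wanders to random navigable points and chases any pawn it sees.
; PawnSensing sightings start an AI move toward the pawn, with a DoOnce switching to run animation and sprint speed.
; Each sighting restarts a short retriggerable delay, so losing sight restores walk animation and speed, re-arms the sprint and resumes wandering.
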(event `self.ReceiveBeginPlay`
  ;[1 1 1] Walk
  (`self.MoveToRandomLocation`))

(event `MoveToRandomLocation`
  ;[1 1 1] Walk
  (bind _randomlocation (`NavigationSystemV1.K2_GetRandomLocationInNavigableRadius` (`self.K2_GetActorLocation`) 0.0 null null))
  (`|AIMoveTo` self _randomlocation null
    (:`OnSuccess`
      (`self.MoveToRandomLocation`))))

(event `cansprintagain`
  ;[1 1 1] Chases us
  (goto _label :!via `Reset`))

(event `self.PawnSensing.OnSeePawn`
  (params (Pawn :type "Pawn Object Reference"))
  ;[1 1 1] Chases us
  (`|ExecutionSequence`
    (:`then_0`
      (`/Engine/EditorBlueprintResources/StandardMacros.DoOnce` false :!label _label
        (:`Completed`
          (`SkeletalMeshComponent.PlayAnimation` (`self.Mesh`) "/Game/StylizedCreaturesBundle/Animations/Wolf/A_Wolf_Run_Forward.A_Wolf_Run_Forward" false)
          (set `CharacterMovementComponent.MaxWalkSpeed` 600.0 (`self.CharacterMovement`)))))
    (:`then_1`
      (`|AIMoveTo` self (0.0 0.0 0.0) Pawn
        (:`then`
          ;[1 1 1] When we hide it stops chasing and walks again
          (`KismetSystemLibrary.RetriggerableDelay` 2.0)
          (`SkeletalMeshComponent.PlayAnimation` (`self.Mesh`) "/Game/StylizedCreaturesBundle/Animations/Wolf/A_Wolf_Walk_Forward.A_Wolf_Walk_Forward" false)
          (set `CharacterMovementComponent.MaxWalkSpeed` 130.0 (`self.CharacterMovement`))
          (`self.cansprintagain`)
          (`self.MoveToRandomLocation`))))))

(fn `UserConstructionScript`)